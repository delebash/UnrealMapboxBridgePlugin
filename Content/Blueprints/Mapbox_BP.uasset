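; Mapbox actor that builds a landscape and its features from map tile files, with empty event and construction graphs.
; GenerateMapboxLandscape caches tile file names, size and geographic coordinates, then imports the heightmap.
; CreateFeatures feeds the stored coordinates and GeoJSON file name, via the TileHeightmapFileName input, into CreateLandscapeFeatures.
; SelectMap starts the WebControl server by console command and calls RunExe with an empty argument.
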(fn `CreateFeatures`
  (`EditorLandscapeLibrary.CreateLandscapeFeatures` (`KismetStringLibrary.Conv_StringToDouble` (`self.CoordinateX`)) (`KismetStringLibrary.Conv_StringToDouble` (`self.CoordinateY`)) (`KismetStringLibrary.Conv_StringToDouble` (`self.OriginNorthing`)) (`KismetStringLibrary.Conv_StringToDouble` (`self.OriginEasting`)) (`self.HeightMapDirectory`) (`self.TileGeojsonFileName`)))

(fn `GenerateMapboxLandscape`
  (params (LandscapeName :type String) (LandscapeSize :type String) (TileHeightmapFileName :type String) (TileGeojsonFileName :type String) (TileInfoFileName :type String) (originLng :type String) (originLat :type String) (Epsg :type String) (OriginNorthing :type String) (OriginEasting :type String) (PointNorthing :type String) (PointEasting :type String))
  (bind _output_get (set `self.Landscape Name` LandscapeName))
  (bind _output_get_2 (set `self.Landscape Size` LandscapeSize))
  (set `self.OriginLng` originLng)
  (set `self.OriginLat` originLat)
  (set `self.OriginEasting` OriginEasting)
  (set `self.OriginNorthing` OriginNorthing)
  (set `self.CoordinateX` PointNorthing)
  (set `self.CoordinateY` PointEasting)
  (set `self.Epsg` Epsg)
  (bind _output_get_3 (set `self.TileHeightmapFileName` TileHeightmapFileName))
  (set `self.TileInfoFileName` TileInfoFileName)
  (set `self.TileGeojsonFileName` TileGeojsonFileName)
  (`EditorLandscapeLibrary.ImportHeightmap` (`self.HeightMapDirectory`) _output_get _output_get_3 (`KismetStringLibrary.Conv_StringToInt` _output_get_2)))

(fn `SelectMap`
  (`KismetSystemLibrary.ExecuteConsoleCommand` null "WebControl.StartServer" null)
  (`EditorLandscapeLibrary.RunExe` ""))

(fn `UserConstructionScript`)
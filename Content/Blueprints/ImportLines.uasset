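; ImportLines is a spline actor that drapes its points onto static world geometry and builds meshes along the line.
; SnapToGround line-traces vertically through each point against WorldStatic and moves it to the hit location, without checking for a hit.
; A second forward pass removes points with truncated world X at or below zero, shifting indices as it iterates.
; RenderMesh separately adds a spline mesh component per segment, matching positions and tangents.
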(event `RenderMesh`
  (bind _spline (`self.Spline`))
  (bind _spline_2 (`self.Spline`))
  (for _index (range (+ (- (`SplineComponent.GetNumberOfSplinePoints` (`self.Spline`)) 2) 1))
    (bind _returnvalue (`AddComponent|NODE_AddSplineMeshComponent-0`))
    (`SplineMeshComponent.SetForwardAxis` _returnvalue "X" true)
    (bind _returnvalue_2 (+ _index 1))
    (`SplineMeshComponent.SetStartAndEnd` _returnvalue (`SplineComponent.GetLocationAtSplinePoint` _spline _index "Local") (`SplineComponent.GetTangentAtSplinePoint` _spline _index "Local") (`SplineComponent.GetLocationAtSplinePoint` _spline_2 _returnvalue_2 "Local") (`SplineComponent.GetTangentAtSplinePoint` _spline_2 _returnvalue_2 "Local") true)))

(event `SnapToGround`
  (bind _spline (`self.Spline`))
  (bind _spline_2 (`self.Spline`))
  (for _index (range (+ (`SplineComponent.GetNumberOfSplinePoints` _spline) 1))
    (bind _x (.x (`SplineComponent.GetLocationAndTangentAtSplinePoint` _spline _index "World")))
    (bind _y (.y (`SplineComponent.GetLocationAndTangentAtSplinePoint` _spline _index "World")))
    (bind _returnvalue (`KismetMathLibrary.MakeVector` _x _y (`KismetMathLibrary.Conv_IntToDouble` 6500000)))
    (`SplineComponent.SetLocationAtSplinePoint` _spline _index _returnvalue "World" true)
    (bind _outhit (`KismetSystemLibrary.LineTraceSingleForObjects` _returnvalue (`KismetMathLibrary.MakeVector` _x _y (`KismetMathLibrary.Conv_IntToDouble` -6500000)) (`|MakeArray` "ObjectTypeQuery1" :!type "EObjectTypeQuery Enum")))
    (`SplineComponent.SetLocationAtSplinePoint` (`self.Spline`) _index (`KismetMathLibrary.MakeVector` (.x (`.Location` (`GameplayStatics.BreakHitResult` _outhit))) (.y (`.Location` (`GameplayStatics.BreakHitResult` _outhit))) (+ (.z (`.Location` (`GameplayStatics.BreakHitResult` _outhit))) 0.0)) "World" true))
  (for _index_2 (range (+ (`SplineComponent.GetNumberOfSplinePoints` _spline_2) 1))
    (if (<= (`KismetMathLibrary.FTrunc` (.x (`SplineComponent.GetLocationAndTangentAtSplinePoint` _spline_2 _index_2 "World"))) 0)
      (`SplineComponent.RemoveSplinePoint` (`self.Spline`) _index_2 true))))

(fn `UserConstructionScript`)